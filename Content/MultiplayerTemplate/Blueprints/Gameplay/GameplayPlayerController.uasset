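; Player controller for the gameplay map in a multiplayer template, handling the local player's UI.
; InitialSetup clears existing widgets, creates the gameplay menu and shows the mouse cursor.
; PrepareForServerTravel has the MultiplayerTemplate game instance show a loading screen before travel.
; SpawnCountdownTime adds a countdown widget to the viewport, seeded with the given number of seconds.
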(event Custom|ShowGameplayMenu
  ;[1 1 1] Show Lobby Menu
  (Viewport|RemoveAllWidgets)
  (UserInterface|CreateWidget "/Game/MultiplayerTemplate/Blueprints/Gameplay/WBP_GameplayMenu.WBP_GameplayMenu_C" self)
  (bind _output_get (Variables|Default|SetWBP_GameplayMenu 0))
  (UserInterface|Viewport|AddtoViewport _output_get 0)
  (Variables|Default|SetbShowMouseCursor true))

(event Custom|PrepareForServerTravel
  ;[1 1 1] Prepare For Server Travel
  (bind _asmultiplayer_template_game_instance (Utilities|Casting|CastToMultiplayerTemplateGameInstance (Game|GetGameInstance)))
  (Default|ShowLoadingScreen _asmultiplayer_template_game_instance))

(event Custom|InitialSetup
  ;[1 1 1] Initial Setup
  (CallFunction|ShowGameplayMenu)
  (Development|PrintString "initGPPC"))

(event Custom|SpawnCountdownTime
  (params (Seconds :type Integer))
  ;[1 1 1] Show Countdown Timer
  (bind _returnvalue (UserInterface|CreateWidget "/Game/MultiplayerTemplate/Blueprints/Lobby/WBP_Countdown_Time.WBP_Countdown_Time_C" self Seconds))
  (UserInterface|Viewport|AddtoViewport _returnvalue 0))

(fn ConstructionScript)