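; Player controller for the multiplayer lobby that sets up the player's menu and lobby identity.
; InitialSetup creates and displays WBP_LobbyMenu, then copies PlayerInfo from the game instance into the LobbyPlayerState.
; UpdatePlayerList finds the menu through a widget class search instead of the stored reference and refreshes its list.
; Its validity check only selects a debug print, so the refresh call runs either way.
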(event Custom|ShowLobbyMenu
  ;[1 1 1] Show Lobby Menu
  (bind _returnvalue (UserInterface|CreateWidget "/Game/MultiplayerTemplate/Blueprints/Lobby/WBP_LobbyMenu.WBP_LobbyMenu_C" self))
  (bind _output_get (Variables|Default|SetWBP_LobbyMenu _returnvalue))
  (UserInterface|Viewport|AddtoViewport _output_get 0))

(event Custom|UpdatePlayerList
  (bind _foundwidgets (Widget|GetAllWidgetsOfClass "/Game/MultiplayerTemplate/Blueprints/Lobby/WBP_LobbyMenu.WBP_LobbyMenu_C" true))
  (Utilities|IsValid (Utilities|Array|Get(acopy) _foundwidgets)
    (:Is%20Valid
      (Development|PrintString "LPC"))
    (:Is%20Not%20Valid
      (Development|PrintString "invalid")))
  (Default|UpdatePlayerList (Utilities|Array|Get(acopy) _foundwidgets))
  (Development|PrintString "End"))

(event Custom|InitialSetup
  ;[1 1 1] Initial Setup
  (CallFunction|ShowLobbyMenu)
  (CallFunction|SetupLobbyPlayerState))

(event Custom|SetupLobbyPlayerState
  ;[1 1 1] Setup Lobby Playerstate
  (bind _asmultiplayer_template_game_instance (Utilities|Casting|CastToMultiplayerTemplateGameInstance (Game|GetGameInstance)))
  (bind _aslobby_player_state (Utilities|Casting|CastToLobbyPlayerState (Variables|GetPlayerState)))
  (Variables|/Game/MultiplayerTemplate/Blueprints/Lobby/LobbyPlayerState.LobbyPlayerState_C|SetPlayerInfo _aslobby_player_state (Variables|/Game/MultiplayerTemplate/Blueprints/AllLevels/MultiplayerTemplateGameInstance.MultiplayerTemplateGameInstance_C|GetPlayerInfo _asmultiplayer_template_game_instance)))

(fn ConstructionScript)